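; Mud is a short-lived actor that can sprout a Root where it sits before disappearing.
; The construction script randomly picks one of two static meshes for its appearance.
; On BeginPlay it waits a few seconds, spawns a Root at its own location on a roughly one-in-three random roll, then destroys itself.
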(event EventBeginPlay
  (Utilities|FlowControl|Delay 3.0)
  (if (< (Math|Random|RandomFloatinRange 0.0 1e+02) 3e+01)
    (Game|SpawnActorfromClass "/Game/ggj2023/Blueprints/Roots/Root.Root_C" (Math|Transform|MakeTransform (Transformation|GetActorLocation) "0, 0, 0" "1.000000,1.000000,1.000000") "Undefined" 0 0))
  (Actor|DestroyActor))

(event Collision|EventActorBeginOverlap
  (params (OtherActor :type Actor%20Object%20Reference)))

(event EventTick
  (params (DeltaSeconds :type Float%20%28single-precision%29)))

(fn ConstructionScript
  (Components|StaticMesh|SetStaticMesh (Variables|Default|GetMud) (select (Math|Random|RandomBool) "/Game/ggj2023/Art/3D/Modelos/Lama_2.Lama_2" "/Game/ggj2023/Art/3D/Modelos/Lama_1.Lama_1")))