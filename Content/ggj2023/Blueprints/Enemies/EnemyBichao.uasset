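; Enemy that chases the player, deals contact damage and, on death, grants XP with a chance to drop a Root actor.
; Tick issues SimpleMoveToActor every frame, bypassing the IsSeeingPlayer check that PawnSensing feeds.
; Sphere overlap damages the player character's PlayerHealth and prints the remaining health.
; Its own PlayerHealth component starts at Vida and drives the death event, which destroys the actor.
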(event OnSeePawn(PawnSensing)
  (params (Pawn :type Pawn%20Object%20Reference))
  (Variables|Default|SetIsSeeingPlayer? true)
  (CallFunction|FollowPlayer))

(event OnComponentBeginOverlap(Sphere)
  (params (OverlappedComponent :type Primitive%20Component%20Object%20Reference) (OtherActor :type Actor%20Object%20Reference) (OtherComp :type Primitive%20Component%20Object%20Reference) (OtherBodyIndex :type Integer) (bFromSweep :type Boolean) (SweepResult :type Hit%20Result%20Structure%20%28by%20ref%29))
  (bind _asbp_top_down_character (Utilities|Casting|CastToBP_TopDownCharacter OtherActor))
  (Default|TakeDamage (Variables|/Game/TopDown/Blueprints/BP_TopDownCharacter.BP_TopDownCharacter_C|GetPlayerHealth _asbp_top_down_character) (Variables|Default|GetDano))
  (Development|PrintString (Utilities|String|ToString(Float) (Variables|/Game/ggj2023/Blueprints/Characters/PlayerHealth.PlayerHealth_C|GetHealth (Variables|/Game/TopDown/Blueprints/BP_TopDownCharacter.BP_TopDownCharacter_C|GetPlayerHealth _asbp_top_down_character)))))

(event EventPlayerDied(PlayerHealth)
  (bind _asbp_top_down_character (Utilities|Casting|CastToBP_TopDownCharacter (Game|GetPlayerCharacter 0)))
  (Default|GainXP _asbp_top_down_character 1)
  (if (< (Math|Random|RandomFloatinRange 0.0 1e+02) 3e+01)
    (Game|SpawnActorfromClass "/Game/ggj2023/Blueprints/Roots/Root.Root_C" (Math|Transform|MakeTransform (Transformation|GetActorLocation) "0, 0, 0" "1.000000,1.000000,1.000000") "Undefined" 0 0))
  (Actor|DestroyActor))

(event Custom|FollowPlayer
  (if (Variables|Default|GetIsSeeingPlayer?)
    (AI|Navigation|SimpleMovetoActor (Pawn|GetController) (Game|GetPlayerCharacter 0))))

(event EventBeginPlay
  (Variables|/Game/ggj2023/Blueprints/Characters/PlayerHealth.PlayerHealth_C|SetHealth (Variables|Default|GetPlayerHealth) (Variables|Default|GetVida)))

(event Collision|EventActorBeginOverlap
  (params (OtherActor :type Actor%20Object%20Reference)))

(event EventTick
  (params (DeltaSeconds :type Float%20%28single-precision%29))
  (AI|Navigation|SimpleMovetoActor (Pawn|GetController) (Game|GetPlayerCharacter 0)))

(fn ConstructionScript)