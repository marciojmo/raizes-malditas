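; PlayerHealth tracks the player's health and signals when the player dies.
; TakeDamage subtracts damage without clamping and calls the PlayerDied event dispatcher whenever health is at or below zero, with no guard against repeat calls.
; RestoreHealth adds health clamped between zero and MaxHealth, and Reset refills it to MaxHealth.
; The event graph is unused, so all logic runs through these three functions.
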(event EventBeginPlay)

(event EventTick
  (params (DeltaSeconds :type Float%20%28single-precision%29)))

(fn TakeDamage
  (params (damage :type Float%20%28double-precision%29))
  (bind _output_get (Variables|Default|SetHealth (- (Variables|Default|GetHealth) damage)))
  (if (<= _output_get 0.0)
    (Default|CallEventPlayerDied)))

(fn Reset
  (Variables|Default|SetHealth (Variables|Default|GetMaxHealth)))

(fn RestoreHealth
  (params (health :type Float%20%28double-precision%29))
  (Variables|Default|SetHealth (Math|Float|Clamp(Float) (+ health (Variables|Default|GetHealth)) 0.0 (Variables|Default|GetMaxHealth))))